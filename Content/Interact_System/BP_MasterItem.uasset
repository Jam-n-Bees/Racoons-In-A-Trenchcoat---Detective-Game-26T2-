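; Base interactable item that shows an interact prompt and outline when the first-person character is near.
; Sphere1 overlaps create and remove a UI_Interact widget on the Widget component, playing its PopUp animation and toggling HintVisible and CanPressE.
; CanReceiveTrace also toggles that prompt state on an existing widget.
; Outlines use an overlay material, applied to Sphere by overlaps and StaticMesh by CanReceiveTrace.
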(event `self.Sphere1.OnComponentBeginOverlap`
  (params (OverlappedComponent :type "PrimitiveComponent Object Reference") (OtherActor :type "Actor Object Reference") (OtherComp :type "PrimitiveComponent Object Reference") (OtherBodyIndex :type Integer) (bFromSweep :type Boolean) (SweepResult :type "HitResult Structure (by ref)"))
  (bind _widget (`self.Widget`))
  (cast `/Game/FirstPerson/Blueprints/BP_FirstPersonCharacter` OtherActor)
  (if (`self.CanInteract`)
    (bind _returnvalue (`|CreateWidget` "/Game/Interact_System/UI_Interact.UI_Interact_C"))
    (bind _output_get (set `self.InteractionWidget` _returnvalue))
    (`WidgetComponent.SetWidget` _widget _output_get)
    (`SceneComponent.SetVisibility` _widget true false)
    (bind _interactionwidget (`self.InteractionWidget`)
      (:`then`
        (if (not (`self.HintVisible`))
          (`UserWidget.PlayAnimation` _interactionwidget (`/Game/Interact_System/UI_Interact.PopUp` _interactionwidget) 0.0 1 "Forward" 1.5 false)
          (set `self.HintVisible` true)
          (`MeshComponent.SetOverlayMaterial` (`self.Sphere`) "/Game/Interact_System/M_OutlineMaterial.M_OutlineMaterial")
          (set `self.CanPressE` true)
          (`KismetSystemLibrary.PrintString` "meow")))
      (:`else`))))

(event `self.Sphere1.OnComponentEndOverlap`
  (params (OverlappedComponent :type "PrimitiveComponent Object Reference") (OtherActor :type "Actor Object Reference") (OtherComp :type "PrimitiveComponent Object Reference") (OtherBodyIndex :type Integer))
  (cast `/Game/FirstPerson/Blueprints/BP_FirstPersonCharacter` OtherActor)
  (`MeshComponent.SetOverlayMaterial` (`self.Sphere`) null)
  (if (`self.CanInteract`)
    (bind _interactionwidget (`self.InteractionWidget`)
      (:`then`
        (if (`self.HintVisible`)
          (`UserWidget.PlayAnimation` _interactionwidget (`/Game/Interact_System/UI_Interact.PopUp` _interactionwidget) 0.0 1 "Forward" 1.5 false)
          (set `self.HintVisible` false)
          (set `self.CanPressE` false)
          (`MeshComponent.SetOverlayMaterial` (`self.Sphere`) null))
        (`KismetSystemLibrary.Delay` 0.15)
        (`Widget.RemoveFromParent` (`self.InteractionWidget`))
        (set `self.InteractionWidget` null)
        (`SceneComponent.SetVisibility` (`self.Widget`) false false)
        (set `self.CanPressE` false)
        (`KismetSystemLibrary.PrintString` "woof"))
      (:`else`))))

(event `/Game/Interact_System/BPI_Interaction.Can Receive Trace`
  (params (`Can Interact` :type Boolean))
  (if (`self.CanInteract`)
    (if `Can Interact`
      (bind _interactionwidget (`self.InteractionWidget`)
        (:`then`
          (if (not (`self.HintVisible`))
            (`UserWidget.PlayAnimation` _interactionwidget (`/Game/Interact_System/UI_Interact.PopUp` _interactionwidget) 0.0 1 "Forward" 1.5 false)
            (set `self.HintVisible` true)
            (`MeshComponent.SetOverlayMaterial` (`self.StaticMesh`) "/Game/Interact_System/M_OutlineMaterial.M_OutlineMaterial")
            (set `self.CanPressE` true)
            (`KismetSystemLibrary.PrintString` "meow 2")))
        (:`else`))
      (else
        (`MeshComponent.SetOverlayMaterial` (`self.StaticMesh`) null)
        (bind _interactionwidget_2 (`self.InteractionWidget`)
          (:`then`
            (if (`self.HintVisible`)
              (`UserWidget.PlayAnimation` _interactionwidget_2 (`/Game/Interact_System/UI_Interact.PopUp` _interactionwidget_2) 0.0 1 "Reverse" 1.5 false)
              (set `self.HintVisible` false)
              (`MeshComponent.SetOverlayMaterial` (`self.StaticMesh`) null)
              (set `self.CanPressE` false)
              (`KismetSystemLibrary.PrintString` "woof 2")))
          (:`else`))))))

(fn `UserConstructionScript`)