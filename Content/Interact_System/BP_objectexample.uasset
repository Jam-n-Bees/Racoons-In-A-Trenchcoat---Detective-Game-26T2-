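; BP_objectexample is an example interactable object in the Interact System that is consumed on use.
; Its custom event runs only while both CanPressE and CanInteract are true.
; It then clears CanInteract to block repeat use, increments and prints the ObligatoryCheck counter, and destroys the actor.
; The construction script only calls its parent.
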(event `CustomEvent_1`
  (bind _obligatory_check (`self.obligatory check`))
  (if (`self.CanPressE`)
    (if (`self.CanInteract`)
      (set `self.CanInteract` false)
      (set `self.obligatory check` (+ _obligatory_check 1))
      (`KismetSystemLibrary.PrintString` (`KismetStringLibrary.Conv_IntToString` _obligatory_check))
      (`self.K2_DestroyActor`))))

(fn `UserConstructionScript`
  (`parent.UserConstructionScript`))