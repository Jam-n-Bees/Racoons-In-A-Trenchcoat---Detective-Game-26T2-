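; Game instance Blueprint, by its name, that saves and restores an item's found state through an SG_Items save object.
; SaveGame creates a fresh save object, copies Item2's Found flag into it and writes it to one slot.
; MenuLoadGame sets a load flag, calls GameLoad to cache the slot's save and switches to game-only input.
; A separate LoadGame function, not called here, copies the cached flag back to Item2.
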(event `MenuLoadGame`
  (set `self.LoadGame?` true)
  (`self.GameLoad`)
  (`WidgetBlueprintLibrary.SetInputMode_GameOnly` (`GameplayStatics.GetPlayerController` 0)))

(fn `GameLoad`
  (bind _returnvalue (`GameplayStatics.LoadGameFromSlot` (`self.SaveSlot1`)))
  (bind _assg_items (cast `/Game/IE_Blueprints/saving/SG_Items` _returnvalue))
  (set `self.SaveRef` _assg_items)
  (return))

(fn `LoadGame`
  (set `/Game/IE_Blueprints/Interaction/Items/BP_ItemExample.Found` (`/Game/IE_Blueprints/saving/SG_Items.Found_2` (`self.SaveRef`)) (`self.item_2`)))

(fn `SaveGame`
  (bind _returnvalue (`GameplayStatics.CreateSaveGameObject` "/Game/IE_Blueprints/saving/SG_Items.SG_Items_C"))
  ; repeat for objects
  (bind _output_get (set `self.SaveRef` _returnvalue))
  (set `/Game/IE_Blueprints/saving/SG_Items.Found_2` (`/Game/IE_Blueprints/Interaction/Items/BP_ItemExample.Found` (`self.item_2`)) _output_get)
  (`GameplayStatics.SaveGameToSlot` (`self.SaveRef`) (`self.SaveSlot1`)))