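; Example child item Blueprint that responds to the Interact event the first time it is triggered.
; On that first interaction it plays the Files sound in 2D, sets the Found flag and prints a debug greeting; later calls do nothing while the flag stays set.
; The construction script only calls the parent, and the BeginPlay and overlap events are disabled stubs.
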(event `/Game/IE_Blueprints/Interaction/BPI_Interact.Interact`
  (if (not (`self.Found`))
    (`GameplayStatics.PlaySound2D` "/Game/sounds/files.files" 1.0 1.0 0.0 null null)
    (set `self.Found` true)
    (`KismetSystemLibrary.PrintString` "Hello")))

(fn `UserConstructionScript`
  (`parent.UserConstructionScript`))