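; Quest flag Blueprint that looks up per-item event flags and handles save and load for eight findable items.
; GetEventHasHappened searches EventsArray by item, but SetEventHasHappened's write logic is disconnected.
; MenuLoadGame calls LoadGame, which reads the SG_Items slot, then clears every Found flag instead of restoring saved values, before game-only input is set.
; SaveGame only creates an SG_Items object, as its slot write is unwired.
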(event `MenuLoadGame`
  (set `self.LoadGame?` true)
  (`self.LoadGame`)
  (`WidgetBlueprintLibrary.SetInputMode_GameOnly` (`GameplayStatics.GetPlayerController` 0)))

(fn `GetEventHasHappened`
  (params (ItemToFind :type "/Game/Programmer/BP_EventClassFlag Object Reference"))
  (returns (EventHasHappened :type Boolean))
  (bind _eventsarray (`self.EventsArray`))
  (return (`/Game/Programmer/BP_EventClassFlag.EventHasHappened` (`|GetArrayItem` _eventsarray (`KismetArrayLibrary.Array_Find` _eventsarray ItemToFind)))))

(fn `LoadGame`
  (bind _returnvalue (`GameplayStatics.LoadGameFromSlot` (`self.SaveSlot`)))
  (bind _assg_items (cast `/Game/IE_Blueprints/SG_Items` _returnvalue))
  (set `self.SaveRef` _assg_items)
  (set `/Game/Placeables/BP_ItemExample.Found` false (`self.ItemEvidence`))
  (set `/Game/Placeables/BP_ItemExample.Found` false (`self.ItemGlass`))
  (set `/Game/Placeables/BP_ItemExample.Found` false (`self.ItemGun`))
  (set `/Game/Placeables/BP_ItemExample.Found` false (`self.ItemLipstick`))
  (set `/Game/Placeables/BP_ItemExample.Found` false (`self.ItemPhotoFrame`))
  (set `/Game/Placeables/BP_ItemExample.Found` false (`self.ItemPillBottle`))
  (set `/Game/Placeables/BP_ItemExample.Found` false (`self.ItemRoomba`))
  (set `/Game/Placeables/BP_ItemExample.Found` false (`self.ItemSword`))
  (return))

(fn `SaveGame`
  (bind _returnvalue (`GameplayStatics.CreateSaveGameObject` "/Game/IE_Blueprints/SG_Items.SG_Items_C"))
  (set `self.SaveRef` _returnvalue))

(fn `SetEventHasHappened`
  (params (EventHasHappened :type Boolean) (ItemToFind :type "/Game/Programmer/BP_EventClassFlag Object Reference")))