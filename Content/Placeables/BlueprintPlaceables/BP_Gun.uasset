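; BP_Gun is a placeable gun Blueprint that registers itself with the game's save-game instance.
; On BeginPlay it casts the Game Instance to BP_NewSaveGameInstanceFix, caches that reference and stores itself in the instance's Gun variable.
; It has no other active logic: Tick and overlap events are disabled, and the construction script only calls its parent.
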(event `self.ReceiveBeginPlay`
  (`parent.ReceiveBeginPlay`)
  (bind _asbp_new_save_game_instance_fix (cast `/Game/IE_Blueprints/ui/BP_NewSaveGameInstanceFix` (`GameplayStatics.GetGameInstance`)))
  (bind _output_get (set `self.GameInstanceRef` _asbp_new_save_game_instance_fix))
  (set `/Game/IE_Blueprints/ui/BP_NewSaveGameInstanceFix.Gun` self _output_get))

(fn `UserConstructionScript`
  (`parent.UserConstructionScript`))